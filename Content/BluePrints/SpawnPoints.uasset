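; Spawner Blueprint that repeatedly spawns PoliceOfficer2 "bobbies" at random SpawnPoint actors in the level.
; BeginPlay caches every SpawnPoint actor in an array and sets a short spawn interval.
; Tick uses Delay nodes for a StartDelay wait and to pace spawning while CanSpawn is true.
; Each spawn takes a random point's root transform and gives the new officer its default controller.
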(event EventBeginPlay
  (CallFunction|SetSpawnPoints)
  (Variables|Default|SetSpawnTime 0.2))

(event EventActorBeginOverlap
  (params (OtherActor :type Actor%20Object%20Reference)))

(event EventTick
  (params (DeltaSeconds :type Float%20%28single-precision%29))
  (if (Variables|Default|GetStartDelay)
    (Utilities|FlowControl|Delay 5.0)
    (Variables|Default|SetStartDelay false))
  (if (Variables|Default|GetCanSpawn)
    (Utilities|FlowControl|Delay (Variables|Default|GetSpawnTime))
    (CallFunction|SpawnBobbies)))

(fn ConstructionScript)

(fn SetSpawnPoints
  (bind _outactors (Actor|GetAllActorsOfClass "/Game/BluePrints/SpawnPoint.SpawnPoint_C"))
  (Variables|Default|SetSpawnPoints _outactors))

(fn SpawnBobbies
  (bind _spawnpoints (Variables|Default|GetSpawnPoints))
  (bind _returnvalue (Game|SpawnActorfromClass "/Game/BluePrints/PoliceOfficer2.PoliceOfficer2_C" (Transformation|GetWorldTransform (Variables|/Game/BluePrints/SpawnPoint.SpawnPoint_C|GetDefaultSceneRoot (Utilities|Array|Get(acopy) _spawnpoints (Math|Random|RandomIntegerinRange 0 (Utilities|Array|LastIndex _spawnpoints))))) "Undefined" 0 0))
  (Pawn|SpawnDefaultController _returnvalue))