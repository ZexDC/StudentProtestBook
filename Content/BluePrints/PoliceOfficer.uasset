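; PoliceOfficer is a police officer Blueprint that animates its Batton component swinging up and down.
; Each Tick lerps the baton's world rotation toward a target offset by 45 degrees of pitch.
; When the baton's relative rotation nears that world-space target, the direction flips and a new target is set.
; Forward movement gated on IsDead exists in the graph but is never executed.
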(event EventBeginPlay
  (Variables|Default|SetBattonRotatingDown true)
  (Variables|Default|SetTargetRotation (Math|Rotator|CombineRotators (Transformation|GetWorldRotation (Variables|Default|Getbatton)) (Math|Rotator|MakeRotator 0.0 -45.0 0.0))))

(event EventActorBeginOverlap
  (params (OtherActor :type Actor%20Object%20Reference)))

(event EventTick
  (params (DeltaSeconds :type Float%20%28single-precision%29))
  (if (Math|Rotator|Equal(Rotator) (Variables|/Script/Engine.SceneComponent|GetRelativeRotation (Variables|Default|Getbatton)) (Variables|Default|GetTargetRotation) 0.1)
    (Variables|Default|SetBattonRotatingDown (not (Variables|Default|GetBattonRotatingDown)))
    (if (Variables|Default|GetBattonRotatingDown)
      (Variables|Default|SetTargetRotation (Math|Rotator|CombineRotators (Transformation|GetWorldRotation (Variables|Default|Getbatton)) (Math|Rotator|MakeRotator 0.0 -45.0 0.0)))
      (else
        (Variables|Default|SetTargetRotation (Math|Rotator|CombineRotators (Transformation|GetWorldRotation (Variables|Default|Getbatton)) (Math|Rotator|MakeRotator 0.0 45.0 0.0)))))
    (else
      (Transformation|SetWorldRotation (Variables|Default|Getbatton) (Math|Rotator|Lerp(Rotator) (Transformation|GetWorldRotation (Variables|Default|Getbatton)) (Variables|Default|GetTargetRotation) 0.2) false false))))

(fn ConstructionScript)