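; Police officer enemy pawn that walks forward, swings a baton and kills the player on contact.
; Tick feeds movement along the control rotation and lerps the baton toward a target pitch offset, flipping direction on arrival for a back-and-forth swing.
; Hitting the player character destroys the officer and calls the player's Death, while a projectile hit or the IsDead flag just removes the officer.
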(event Collision|EventHit
  (params (MyComp :type Primitive%20Component%20Object%20Reference) (Other :type Actor%20Object%20Reference) (OtherComp :type Primitive%20Component%20Object%20Reference) (bSelfMoved :type Boolean) (HitLocation :type Vector :default "0, 0, 0") (HitNormal :type Vector :default "0, 0, 0") (NormalImpulse :type Vector :default "0, 0, 0") (Hit :type Hit%20Result%20Structure%20%28by%20ref%29))
  (bind _returnvalue (Utilities|GetClass Other))
  (if (Utilities|ClassIsChildOf _returnvalue "/Game/FirstPersonBP/Blueprints/FpsCharacterMain.FpsCharacterMain_C")
    (Rendering|SetActorHiddenInGame true)
    (Actor|DestroyActor)
    (bind _asfps_character_main (Utilities|Casting|CastToFpsCharacterMain Other))
    (Default|Death _asfps_character_main)
    (elif (Utilities|ClassIsChildOf _returnvalue "/Game/FirstPersonBP/Blueprints/FirstPersonProjectile.FirstPersonProjectile_C")
      (Rendering|SetActorHiddenInGame true)
      (Actor|DestroyActor))))

(event EventTick
  (params (DeltaSeconds :type Float%20%28single-precision%29))
  (if (Variables|Default|GetIsDead)
    (Actor|DestroyActor)
    (else
      (Utilities|FlowControl|Sequence
        (:then_0
          (Pawn|Input|AddMovementInput (Math|Vector|GetForwardVector (Pawn|GetControlRotation :!class /Script/Engine.Pawn)) 1.0 false))
        (:then_1
          (if (Math|Rotator|Equal(Rotator) (Transformation|GetWorldRotation (Variables|Default|Getbatton)) (Variables|Default|GetTargetRotation) 0.1)
            (bind _output_get (Variables|Default|SetBattonRotatingDown (not (Variables|Default|GetBattonRotatingDown))))
            (if _output_get
              (Variables|Default|SetTargetRotation (Math|Rotator|CombineRotators (Transformation|GetWorldRotation (Variables|Default|Getbatton)) (Math|Rotator|MakeRotator 0.0 -45.0 0.0)))
              (else
                (Variables|Default|SetTargetRotation (Math|Rotator|CombineRotators (Transformation|GetWorldRotation (Variables|Default|Getbatton)) (Math|Rotator|MakeRotator 0.0 45.0 0.0)))))
            (else
              (Transformation|SetWorldRotation (Variables|Default|Getbatton) (Math|Rotator|Lerp(Rotator) (Transformation|GetWorldRotation (Variables|Default|Getbatton)) (Variables|Default|GetTargetRotation) 0.2) false false))))))))

(event EventBeginPlay
  (Variables|Default|SetBattonRotatingDown true)
  (Variables|Default|SetTargetRotation (Math|Rotator|CombineRotators (Transformation|GetWorldRotation (Variables|Default|Getbatton)) (Math|Rotator|MakeRotator 0.0 -45.0 0.0))))

(fn ConstructionScript)